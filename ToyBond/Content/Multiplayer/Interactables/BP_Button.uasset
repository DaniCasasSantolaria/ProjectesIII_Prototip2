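; BP_Button is an interactable button that triggers a linked object when a BP_Axe hits its plate.
; Interact plays a timeline that slides the plate along X and sends StartInteractionMessage to ObjectToInteract; StopInteract reverses both.
; BeginPlay resets the plate and clears any linked object lacking BPI_InteractableObject.
; InteractZone overlaps only cast to BP_Firefighter, and nothing here calls StopInteract.
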(event OnComponentHit(Plate)
  (params (HitComponent :type Primitive%20Component%20Object%20Reference) (OtherActor :type Actor%20Object%20Reference) (OtherComp :type Primitive%20Component%20Object%20Reference) (NormalImpulse :type Vector :default "0, 0, 0") (Hit :type Hit%20Result%20Structure%20%28by%20ref%29))
  (Utilities|Casting|CastToBP_Axe OtherActor)
  (CallFunction|Interact))

(event OnComponentBeginOverlap(InteractZone)
  (params (OverlappedComponent :type Primitive%20Component%20Object%20Reference) (OtherActor :type Actor%20Object%20Reference) (OtherComp :type Primitive%20Component%20Object%20Reference) (OtherBodyIndex :type Integer) (bFromSweep :type Boolean) (SweepResult :type Hit%20Result%20Structure%20%28by%20ref%29))
  (Utilities|Casting|CastToBP_Firefighter OtherActor))

(event OnComponentEndOverlap(InteractZone)
  (params (OverlappedComponent :type Primitive%20Component%20Object%20Reference) (OtherActor :type Actor%20Object%20Reference) (OtherComp :type Primitive%20Component%20Object%20Reference) (OtherBodyIndex :type Integer))
  (Utilities|Casting|CastToBP_Firefighter OtherActor))

(event Custom|Stop%20Button%20Anim
  (bind _plate (Variables|Default|GetPlate))
  (bind _relativelocation (Variables|/Script/Engine.SceneComponent|GetRelativeLocation _plate))
  ;[0.5677 0.5677 0.5677 0.5] Button Animation
  (bind _height (Timeline|PlateAnim Stop)
    (:Update
      (Transformation|SetRelativeLocation (Variables|Default|GetPlate) (Math|Vector|MakeVector (Math|Float|Lerp (Variables|Default|GetNotActivePositionX) (Variables|Default|GetActivePositionX) _height) (.y _relativelocation) (.z _relativelocation)) false false))))

(event Custom|Start%20Button%20Animation
  (bind _plate (Variables|Default|GetPlate))
  (bind _relativelocation (Variables|/Script/Engine.SceneComponent|GetRelativeLocation _plate))
  ;[0.5677 0.5677 0.5677 0.5] Button Animation
  (bind _height (Timeline|PlateAnim Play)
    (:Update
      (Transformation|SetRelativeLocation (Variables|Default|GetPlate) (Math|Vector|MakeVector (Math|Float|Lerp (Variables|Default|GetNotActivePositionX) (Variables|Default|GetActivePositionX) _height) (.y _relativelocation) (.z _relativelocation)) false false))))

(event Custom|Reverse%20Button%20Animation
  (bind _plate (Variables|Default|GetPlate))
  (bind _relativelocation (Variables|/Script/Engine.SceneComponent|GetRelativeLocation _plate))
  ;[0.5677 0.5677 0.5677 0.5] Button Animation
  (bind _height (Timeline|PlateAnim Reverse)
    (:Update
      (Transformation|SetRelativeLocation (Variables|Default|GetPlate) (Math|Vector|MakeVector (Math|Float|Lerp (Variables|Default|GetNotActivePositionX) (Variables|Default|GetActivePositionX) _height) (.y _relativelocation) (.z _relativelocation)) false false))))

(event EventStopInteract
  (CallFunction|ReverseButtonAnimation)
  (bind _object_to_interact (Variables|Default|GetObject%20To%20Interact)
    (:then
      (Class|BPIInteractableObject|ReverseInteraction(Message) _object_to_interact))
    (:else)))

(event EventInteract
  (CallFunction|StartButtonAnimation)
  (bind _object_to_interact (Variables|Default|GetObject%20To%20Interact)
    (:then
      (Class|BPIInteractableObject|StartInteraction(Message) _object_to_interact))
    (:else)))

(event EventBeginPlay
  (bind _plate (Variables|Default|GetPlate))
  (bind _relativelocation (Variables|/Script/Engine.SceneComponent|GetRelativeLocation _plate))
  (Transformation|SetRelativeLocation (Variables|Default|GetPlate) (Math|Vector|MakeVector (Variables|Default|GetNotActivePositionX) (.y _relativelocation) (.z _relativelocation)) false true)
  (CallFunction|StopButtonAnim)
  (bind _object_to_interact (Variables|Default|GetObject%20To%20Interact)
    (:then
      (if (not (Utilities|DoesObjectImplementInterface _object_to_interact "/Game/Multiplayer/InteractableObjects/BPI_InteractableObject.BPI_InteractableObject_C"))
        (Variables|Default|SetObject%20To%20Interact 0)))
    (:else)))

(fn ConstructionScript)