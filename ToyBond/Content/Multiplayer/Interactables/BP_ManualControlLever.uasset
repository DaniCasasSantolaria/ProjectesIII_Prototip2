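; BP_ManualControlLever is an interactable lever that triggers a list of target objects and tilts with player axis input.
; On BeginPlay it filters ObjectsToInteract by BPI_InteractableObject, then Interact and StopInteract send those targets start and reverse interaction messages.
; While in use, SetInteractAxis maps input to a clamped pitch between MinAngle and MaxAngle on RotationPoint.
; The axis value only rotates the lever and is not forwarded to the targets.
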(event EventInteract
  (Variables|Default|SetIs%20Being%20Used true)
  (for _array_element (Variables|Default|GetObjects%20To%20Interact)
    (Class|BPIInteractableObject|StartInteraction(Message) _array_element)))

(event EventStopInteract
  (Variables|Default|SetIs%20Being%20Used false)
  (for _array_element (Variables|Default|GetObjects%20To%20Interact)
    (Class|BPIInteractableObject|ReverseInteraction(Message) _array_element)))

(event EventSetInteractAxis
  (params (Axis%20Value :type Float%20%28double-precision%29))
  (if (Variables|Default|GetIs%20Being%20Used)
    (bind _output_get (Variables|Default|SetLever%20Angle (Math|Float|MapRangeClamped Axis%20Value -1.0 1.0 (Variables|Default|GetMin%20Angle) (Variables|Default|GetMax%20Angle))))
    (Transformation|SetRelativeRotation (Variables|Default|GetRotationPoint) (Math|Rotator|MakeRotator 0.0 _output_get 0.0) false false)))

(event EventBeginPlay
  (for _array_element (Variables|Default|GetObjects%20To%20Interact)
    (if (not (Utilities|DoesObjectImplementInterface _array_element "/Game/Multiplayer/InteractableObjects/BPI_InteractableObject.BPI_InteractableObject_C"))
      (Utilities|Array|RemoveItem (Variables|Default|GetObjects%20To%20Interact) _array_element))))

(fn ConstructionScript)