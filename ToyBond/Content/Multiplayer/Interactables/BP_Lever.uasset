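; Interactable lever that toggles between two pitch angles and drives a list of linked objects.
; BeginPlay sets the starting pitch and prunes linked objects lacking BPI_InteractableObject.
; Each Interact alternates via FlipFlop, switching the target angle, playing or reversing TimelineRotation, and sending start or reverse interaction messages to the linked objects.
; The timeline's Update serves as a tick, easing RotationPoint toward the target with FInterpTo.
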(event EventInteract
  (Utilities|FlowControl|FlipFlop
    (:A
      (Variables|Default|SetTargetAngle (Variables|Default|GetMin%20Angle))
      (Audio|Components|Audio|Play (Variables|Default|GetTimeline%20Rotation))
      (for _array_element (Variables|Default|GetObjects%20To%20Interact)
        (Class|BPIInteractableObject|StartInteraction(Message) _array_element)))
    (:B
      (Variables|Default|SetTargetAngle (Variables|Default|GetMax%20Angle))
      (Utilities|String|Reverse (Variables|Default|GetTimeline%20Rotation))
      (for _array_element_2 (Variables|Default|GetObjects%20To%20Interact)
        (Class|BPIInteractableObject|ReverseInteraction(Message) _array_element_2)))))

(event EventBeginPlay
  (Variables|Default|SetTargetAngle (Variables|Default|GetMin%20Angle))
  (Transformation|SetRelativeRotation (Variables|Default|GetRotationPoint) (Math|Rotator|MakeRotator 0.0 (Variables|Default|GetMax%20Angle) 0.0) false false)
  (for _array_element (Variables|Default|GetObjects%20To%20Interact)
    (if (not (Utilities|DoesObjectImplementInterface _array_element "/Game/Multiplayer/InteractableObjects/BPI_InteractableObject.BPI_InteractableObject_C"))
      (Utilities|Array|RemoveItem (Variables|Default|GetObjects%20To%20Interact) _array_element))))

(fn ConstructionScript)