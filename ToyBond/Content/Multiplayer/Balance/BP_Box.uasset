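; BP_Box is a physics box in the multiplayer Balance folder that has its own flippable vertical gravity.
; Each Tick applies a Z force to its static mesh from mass, Gravity and GravityScale, flagged as an acceleration change, so acceleration scales with mass.
; ChangeGravityDirection negates GravityScale to reverse the pull.
; GetGravityDirection reports whether the resulting gravity points upward.
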(event EventBeginPlay)

(event Collision|EventActorBeginOverlap
  (params (OtherActor :type Actor%20Object%20Reference)))

(event EventTick
  (params (DeltaSeconds :type Float%20%28single-precision%29))
  (Physics|AddForce (Variables|Default|GetStaticMesh) (Math|Vector|MakeVector 0.0 0.0 (* (Physics|GetMass (Variables|Default|GetStaticMesh)) (Variables|Default|GetGravity) (Variables|Default|GetGravity%20Scale))) "None" true))

(event EventChangeGravityDirection
  (Variables|Default|SetGravity%20Scale (* (Variables|Default|GetGravity%20Scale) -1.0)))

(fn ConstructionScript)

(fn GetGravityDirection
  (return (> (* (Variables|Default|GetGravity) (Variables|Default|GetGravity%20Scale)) 0.0)))