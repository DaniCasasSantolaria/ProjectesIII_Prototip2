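; Balance actor that tilts from the mass of overlapping objects on two sides, with Trigger2 accepting only actors whose gravity-direction interface check returns true.
; Each new overlap replaces that side's mass map, then recalculates target pitch from weight difference and limits, flipping sign on Trigger2's gravity state.
; Tick interpolates RotationZone pitch at a speed scaled by imbalance.
; The construction script scales the balance and positions both zones symmetrically.
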(event OnComponentBeginOverlap(Trigger2)
  (params (OverlappedComponent :type Primitive%20Component%20Object%20Reference) (OtherActor :type Actor%20Object%20Reference) (OtherComp :type Primitive%20Component%20Object%20Reference) (OtherBodyIndex :type Integer) (bFromSweep :type Boolean) (SweepResult :type Hit%20Result%20Structure%20%28by%20ref%29))
  ;[0.15 0.15 0.15 0.5] Down Trigger Logic
  (Utilities|IsValid OtherActor
    (:Is%20Valid
      (Utilities|IsValid OtherComp
        (:Is%20Valid
          (if (Utilities|DoesObjectImplementInterface OtherActor "/Game/Multiplayer/GravityInterface/BPI_GravityInterface.BPI_GravityInterface_C")
            (Variables|Default|SetActor%20Overlaped%20Trigger%202 OtherActor)
            (bind _gravity_up (Class|BPIGravityInterface|GetGravityDirection(Message) (Variables|Default|GetActor%20Overlaped%20Trigger%202)))
            (if _gravity_up
              (Variables|Default|SetOverlap%20Actors%20Right (Utilities|Map|MakeMap OtherActor (Physics|GetMass OtherComp)))
              (CallFunction|RecalculateandUpdate))))))))

(event OnComponentBeginOverlap(Trigger1)
  (params (OverlappedComponent :type Primitive%20Component%20Object%20Reference) (OtherActor :type Actor%20Object%20Reference) (OtherComp :type Primitive%20Component%20Object%20Reference) (OtherBodyIndex :type Integer) (bFromSweep :type Boolean) (SweepResult :type Hit%20Result%20Structure%20%28by%20ref%29))
  ;[0.15 0.15 0.15 0.5] Up Trigger Logic
  (Utilities|IsValid OtherActor
    (:Is%20Valid
      (Utilities|IsValid OtherComp
        (:Is%20Valid
          (Variables|Default|SetActor%20Overlaped%20Trigger%201 OtherActor)
          (Variables|Default|SetOverlap%20Actors%20Left (Utilities|Map|MakeMap OtherActor (Physics|GetMass OtherComp)))
          (CallFunction|RecalculateandUpdate))))))

(event OnComponentEndOverlap(Trigger1)
  (params (OverlappedComponent :type Primitive%20Component%20Object%20Reference) (OtherActor :type Actor%20Object%20Reference) (OtherComp :type Primitive%20Component%20Object%20Reference) (OtherBodyIndex :type Integer))
  ;[0.15 0.15 0.15 0.5] Up Trigger Logic
  (Utilities|IsValid OtherActor
    (:Is%20Valid
      (Utilities|IsValid OtherComp
        (:Is%20Valid
          (Variables|Default|SetActor%20Overlaped%20Trigger%201 0)
          (Utilities|Map|Remove (Variables|Default|GetOverlap%20Actors%20Left) OtherActor)
          (CallFunction|RecalculateandUpdate))))))

(event OnComponentEndOverlap(Trigger2)
  (params (OverlappedComponent :type Primitive%20Component%20Object%20Reference) (OtherActor :type Actor%20Object%20Reference) (OtherComp :type Primitive%20Component%20Object%20Reference) (OtherBodyIndex :type Integer))
  ;[0.15 0.15 0.15 0.5] Down Trigger Logic
  (Utilities|IsValid OtherActor
    (:Is%20Valid
      (Utilities|IsValid OtherComp
        (:Is%20Valid
          (Variables|Default|SetActor%20Overlaped%20Trigger%202 0)
          (Utilities|Map|Remove (Variables|Default|GetOverlap%20Actors%20Right) OtherActor)
          (CallFunction|RecalculateandUpdate))))))

(event EventTick
  (params (DeltaSeconds :type Float%20%28single-precision%29))
  (bind _rotation_zone (Variables|Default|GetRotation%20Zone))
  (bind _relativerotation (Variables|/Script/Engine.SceneComponent|GetRelativeRotation _rotation_zone))
  (Transformation|SetRelativeRotation (Variables|Default|GetRotation%20Zone) (Math|Rotator|MakeRotator (.roll _relativerotation) (Math|Interpolation|FInterpTo (.pitch (Variables|/Script/Engine.SceneComponent|GetRelativeRotation (Variables|Default|GetRotation%20Zone))) (Variables|Rotation|GetTarget%20Rotation) (Utilities|Time|GetWorldDeltaSeconds) (Variables|Rotation|GetInterp%20Speed)) (.yaw _relativerotation)) false false))

(fn ConstructionScript
  (bind _zone_1 (Variables|Default|GetZone%201))
  (bind _zone_2 (Variables|Default|GetZone%202))
  (bind _relativelocation (Variables|/Script/Engine.SceneComponent|GetRelativeLocation _zone_2))
  (bind _relativelocation_2 (Variables|/Script/Engine.SceneComponent|GetRelativeLocation _zone_1))
  (Transformation|SetRelativeScale3D (Variables|Default|GetBalance) (Variables|Default|GetScale))
  (Transformation|SetRelativeScale3D (Variables|Default|GetZone%201) (Variables|Default|GetZonesScale))
  (Transformation|SetRelativeScale3D (Variables|Default|GetZone%202) (Variables|Default|GetZonesScale))
  (Transformation|SetRelativeLocation (Variables|Default|GetZone%201) (Math|Vector|MakeVector (* (Variables|Default|GetDistance%20Zones%20From%20Center) (.x (Variables|/Script/Engine.SceneComponent|GetRelativeScale3D (Variables|Default|GetBalance)))) (.y _relativelocation_2) (.z _relativelocation_2)) false false)
  (Transformation|SetRelativeLocation (Variables|Default|GetZone%202) (Math|Vector|MakeVector (* (Variables|Default|GetDistance%20Zones%20From%20Center) (.x (Variables|/Script/Engine.SceneComponent|GetRelativeScale3D (Variables|Default|GetBalance))) -1.0) (.y _relativelocation) (.z _relativelocation)) false false))

(fn RecalculateandUpdate
  (Utilities|FlowControl|Sequence
    (:then_0
      (Variables|Weight|SetCurrent%20Weight%20Left 0.0)
      (bind _values (Utilities|Map|Values (Variables|Default|GetOverlap%20Actors%20Left)))
      (for _array_element _values
        (Variables|Weight|SetCurrent%20Weight%20Left (+ _array_element (Variables|Weight|GetCurrent%20Weight%20Left)))))
    (:then_1
      (Variables|Weight|SetCurrent%20Weight%20Right 0.0)
      (bind _values_2 (Utilities|Map|Values (Variables|Default|GetOverlap%20Actors%20Right)))
      (for _array_element_2 _values_2
        (Variables|Weight|SetCurrent%20Weight%20Right (+ _array_element_2 (Variables|Weight|GetCurrent%20Weight%20Right)))))
    (:then_2
      (CallFunction|UpdateBalanceRotation))))

(fn UpdateBalanceRotation
  (Utilities|FlowControl|Sequence
    (:then_0
      (if (and (|CurrentRightWeight>MaxLeftWeight) (|CurrentRightWeight>MaxRightWeight))
        (Variables|Rotation|SetTarget%20Rotation 0.0)
        (elif (and (|CurrentRightWeight>MaxLeftWeight_2) (not (|CurrentRightWeight>MaxRightWeight_2)))
          (Variables|Rotation|SetTarget%20Rotation (Variables|Rotation|GetMax%20Rotation))
          (elif (and (not (|CurrentRightWeight>MaxLeftWeight_2_2)) (|CurrentRightWeight>MaxRightWeight_2_2))
            (Variables|Rotation|SetTarget%20Rotation (Variables|Rotation|GetMax%20Rotation))
            (elif (> (+ (Variables|Weight|GetMax%20Weight%20Left) (Variables|Weight|GetMax%20Weight%20Right)) 0.0001)
              (bind _gravity_up (Class|BPIGravityInterface|GetGravityDirection(Message) (Variables|Default|GetActor%20Overlaped%20Trigger%202)))
              (if _gravity_up
                (Variables|Rotation|SetTarget%20Rotation (* (Math|Float|Clamp(Float) (/ (- (Variables|Weight|GetCurrent%20Weight%20Left) (Variables|Weight|GetCurrent%20Weight%20Right)) (+ (Variables|Weight|GetMax%20Weight%20Left) (Variables|Weight|GetMax%20Weight%20Right))) -1.0) (* (Variables|Rotation|GetMax%20Rotation) -1.0)))
                (else
                  (Variables|Rotation|SetTarget%20Rotation (* (Math|Float|Clamp(Float) (/ (- (Variables|Weight|GetCurrent%20Weight%20Left) (Variables|Weight|GetCurrent%20Weight%20Right)) (+ (Variables|Weight|GetMax%20Weight%20Left) (Variables|Weight|GetMax%20Weight%20Right))) -1.0) (Variables|Rotation|GetMax%20Rotation)))))
              (else
                (Variables|Rotation|SetTarget%20Rotation 0.0)))))))
    (:then_1
      (Variables|Rotation|SetInterp%20Speed (Math|Float|MapRangeClamped (Math|Float|Absolute(Float) (- (Variables|Weight|GetCurrent%20Weight%20Left) (Variables|Weight|GetCurrent%20Weight%20Right))) 0.0 (Math|Float|Max(Float) (Math|Float|SelectFloat (Variables|Weight|GetMax%20Weight%20Left) (Variables|Weight|GetMax%20Weight%20Right) (> (- (Variables|Weight|GetCurrent%20Weight%20Left) (Variables|Weight|GetCurrent%20Weight%20Right)) 0.0)) (Math|Float|MakeLiteralFloat 0.0001)) (Variables|Default|GetMin%20Interp%20Speed) (Variables|Default|GetMax%20Interp%20Speed))))))