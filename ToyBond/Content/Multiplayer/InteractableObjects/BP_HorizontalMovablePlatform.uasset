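; Interactable platform that slides back and forth along world Y, between its start position and a set distance from it.
; StartInteraction sets the MovePlatform timeline's play rate from TimeToMove and plays it on first use, lerping Y with a swept move.
; Stop and reverse interactions both pause it by zeroing the play rate, so a later start resumes in place.
; When the timeline finishes, it flips direction via IsGoingRight, looping continuously.
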(event EventBeginPlay
  (Variables|Position|SetStart%20Location (Transformation|GetActorLocation))
  (Variables|Position|SetMinY%20Position (.y (Variables|Position|GetStart%20Location)))
  (Variables|Position|SetMaxY%20Position (+ (.y (Variables|Position|GetStart%20Location)) (Variables|Default|GetDistance%20To%20Move))))

(event EventReverseInteraction
  (CallFunction|StopInteraction))

(event EventStopInteraction
  (Components|Timeline|SetPlayRate (Variables|Default|GetMove%20Platform) 0.0))

(event EventStartInteraction
  (bind _output_get (Variables|Default|SetPlay%20Rate (/ 1.0 (Variables|Default|GetTimeToMove))))
  (Components|Timeline|SetPlayRate (Variables|Default|GetMove%20Platform) _output_get)
  (if (not (Variables|Default|GetStarted))
    (Components|Timeline|PlayfromStart (Variables|Default|GetMove%20Platform))
    (Variables|Default|SetStarted true)))

(fn ConstructionScript)