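; BP_ChangeGravity is an interactable that changes the gravity direction of non-Pawn actors inside its Box volume.
; Box overlap events maintain an ActorsOverlapped list, admitting only actors that implement BPI_GravityInterface and are not Pawns.
; StartInteraction sends ChangeGravityDirectionMessage to every tracked actor.
; StopInteraction is empty, so ReverseInteraction, which only calls it, has no effect.
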(event OnComponentBeginOverlap(Box)
  (params (OverlappedComponent :type Primitive%20Component%20Object%20Reference) (OtherActor :type Actor%20Object%20Reference) (OtherComp :type Primitive%20Component%20Object%20Reference) (OtherBodyIndex :type Integer) (bFromSweep :type Boolean) (SweepResult :type Hit%20Result%20Structure%20%28by%20ref%29))
  (if (Utilities|DoesObjectImplementInterface OtherActor "/Game/Multiplayer/GravityInterface/BPI_GravityInterface.BPI_GravityInterface_C")
    (Utilities|Casting|CastToPawn OtherActor
      (:CastFailed
        (Utilities|Array|Add (Variables|Default|GetActorsOverlapped) OtherActor)))))

(event OnComponentEndOverlap(Box)
  (params (OverlappedComponent :type Primitive%20Component%20Object%20Reference) (OtherActor :type Actor%20Object%20Reference) (OtherComp :type Primitive%20Component%20Object%20Reference) (OtherBodyIndex :type Integer))
  (if (Utilities|DoesObjectImplementInterface OtherActor "/Game/Multiplayer/GravityInterface/BPI_GravityInterface.BPI_GravityInterface_C")
    (Utilities|Casting|CastToPawn OtherActor
      (:CastFailed
        (Utilities|Array|RemoveItem (Variables|Default|GetActorsOverlapped) OtherActor)))))

(event EventStartInteraction
  (for _array_element (Variables|Default|GetActorsOverlapped)
    (Class|BPIGravityInterface|ChangeGravityDirection(Message) _array_element)))

(event EventStopInteraction)

(event EventReverseInteraction
  (CallFunction|StopInteraction))

(fn ConstructionScript)