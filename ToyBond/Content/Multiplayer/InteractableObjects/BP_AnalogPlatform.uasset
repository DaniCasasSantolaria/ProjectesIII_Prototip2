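; BP_AnalogPlatform is an interactable platform that moves along Y and Z between its start location and configured distances.
; On BeginPlay it registers itself with two child-actor manual control levers, one per axis.
; Move turns a direction into play or reverse on per-axis timelines, whose updates lerp the location with sweep; separate functions stop each axis.
; Reverse and Stop interaction events are empty, and CalculateNewPos is not called here.
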(event EventBeginPlay
  (Variables|Default|SetPlay%20Rate (/ 1.0 (Variables|Default|GetTimeToMove)))
  (Variables|Position|SetStart%20Location (Transformation|GetActorLocation))
  (Variables|Position|SetMinY%20Position (.y (Variables|Position|GetStart%20Location)))
  (Variables|Position|SetMaxY%20Position (+ (.y (Variables|Position|GetStart%20Location)) (Variables|Default|GetDistance%20To%20Move%20Y)))
  (Variables|Position|SetMinZ%20Position (.z (Variables|Position|GetStart%20Location)))
  (Variables|Position|SetMaxZ%20Position (+ (.z (Variables|Position|GetStart%20Location)) (Variables|Default|GetDistance%20To%20Move%20Z)))
  (bind _asbp_manual_control_lever (Utilities|Casting|CastToBP_ManualControlLever (Variables|/Script/Engine.ChildActorComponent|GetChildActor (Variables|Default|GetBP_ManualControlLever%20Z))))
  (Variables|/Game/Multiplayer/Interactables/BP_ManualControlLever.BP_ManualControlLever_C|SetPlatform%20To%20Interact _asbp_manual_control_lever self)
  (bind _asbp_manual_control_lever_2 (Utilities|Casting|CastToBP_ManualControlLever (Variables|/Script/Engine.ChildActorComponent|GetChildActor (Variables|Default|GetBP_ManualControlLever%20Y))))
  (Variables|/Game/Multiplayer/Interactables/BP_ManualControlLever.BP_ManualControlLever_C|SetPlatform%20To%20Interact _asbp_manual_control_lever_2 self))

(event EventReverseInteraction)

(event EventStopInteraction)

(event EventStartInteraction
  (bind _output_get (Variables|Default|SetPlay%20Rate (/ 1.0 (Variables|Default|GetTimeToMove))))
  (Components|Timeline|SetPlayRate (Variables|Default|GetMove%20Platform%20Y) _output_get)
  (Components|Timeline|SetPlayRate (Variables|Default|GetMovePlatform%20%20Z) (/ 1.0 (Variables|Default|GetTimeToMove))))

(fn ConstructionScript)

(fn Move
  (params (Direction :type Vector))
  (Variables|Default|SetDirection%20Y (.y Direction))
  (Variables|Default|SetDirection%20Z (.z Direction))
  (Utilities|FlowControl|Sequence
    (:then_0
      (Components|Timeline|SetPlayRate (Variables|Default|GetMove%20Platform%20Y) (Variables|Default|GetPlay%20Rate))
      (if (> (Variables|Default|GetDirection%20Y) 0.05)
        (Audio|Components|Audio|Play (Variables|Default|GetMove%20Platform%20Y))
        (elif (< (Variables|Default|GetDirection%20Y) 0.05)
          (Utilities|String|Reverse (Variables|Default|GetMove%20Platform%20Y))
          (else
            (Audio|Components|Audio|Stop (Variables|Default|GetMove%20Platform%20Y))))))
    (:then_1
      (Components|Timeline|SetPlayRate (Variables|Default|GetMovePlatform%20%20Z) (Variables|Default|GetPlay%20Rate))
      (if (> (Variables|Default|GetDirection%20Z) 0.05)
        (Audio|Components|Audio|Play (Variables|Default|GetMovePlatform%20%20Z))
        (Development|PrintString "Move")
        (elif (< (Variables|Default|GetDirection%20Z) 0.05)
          (Utilities|String|Reverse (Variables|Default|GetMovePlatform%20%20Z))
          (Development|PrintString "Reverse")
          (else
            (Audio|Components|Audio|Stop (Variables|Default|GetMovePlatform%20%20Z))
            (Development|PrintString "Stop")))))))

(fn StopMoveY
  (Audio|Components|Audio|Stop (Variables|Default|GetMove%20Platform%20Y)))

(fn StopMoveZ
  (Audio|Components|Audio|Stop (Variables|Default|GetMovePlatform%20%20Z)))

(fn CalculateNewPos
  (params (Axis :type Float%20%28double-precision%29) (Moving%20Y :type Boolean))
  (Variables|Default|SetAxis%20Value%20For%20New%20Pos Axis)
  (if Moving%20Y
    (if (> (Variables|Default|GetAxis%20Value%20For%20New%20Pos) 0.0)
      (return (+ (* (Utilities|Time|GetWorldDeltaSeconds) (Variables|Default|GetSpeed) (Variables|Default|GetAxis%20Value%20For%20New%20Pos)) (.y (Transformation|GetActorLocation))))
      (else
        (return (- (* (Utilities|Time|GetWorldDeltaSeconds) (Variables|Default|GetSpeed) (Variables|Default|GetAxis%20Value%20For%20New%20Pos)) (.y (Transformation|GetActorLocation))))))
    (elif (> (Variables|Default|GetAxis%20Value%20For%20New%20Pos) 0.0)
      (return (+ (* (Variables|Default|GetAxis%20Value%20For%20New%20Pos) (Variables|Default|GetSpeed) (Utilities|Time|GetWorldDeltaSeconds)) (.z (Transformation|GetActorLocation))))
      (else
        (return (- (* (Variables|Default|GetAxis%20Value%20For%20New%20Pos) (Variables|Default|GetSpeed) (Utilities|Time|GetWorldDeltaSeconds)) (.z (Transformation|GetActorLocation))))))))