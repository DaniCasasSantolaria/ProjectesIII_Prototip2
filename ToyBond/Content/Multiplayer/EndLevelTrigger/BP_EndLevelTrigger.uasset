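; BP_EndLevelTrigger is a multiplayer end-of-level volume that loads the next level once at least two players stand inside.
; Trigger overlap events count BP_Firefighter and BP_Astronaut actors entering and leaving; a delayed BeginPlay scan also adds already-overlapping astronauts only.
; When an entry brings the count to two, a Fade widget plays before NextLevel opens.
; The construction script sizes the trigger box from BoxExtent.
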(event OnComponentBeginOverlap(Trigger)
  (params (OverlappedComponent :type Primitive%20Component%20Object%20Reference) (OtherActor :type Actor%20Object%20Reference) (OtherComp :type Primitive%20Component%20Object%20Reference) (OtherBodyIndex :type Integer) (bFromSweep :type Boolean) (SweepResult :type Hit%20Result%20Structure%20%28by%20ref%29))
  (Utilities|Casting|CastToBP_Firefighter OtherActor
    (:then
      (Variables|Default|SetAmount%20Players%20overlapped (+ (Variables|Default|GetAmount%20Players%20overlapped) 1)))
    (:CastFailed
      (Utilities|Casting|CastToBP_Astronaut OtherActor)
      (Variables|Default|SetAmount%20Players%20overlapped (+ (Variables|Default|GetAmount%20Players%20overlapped) 1))))
  (if (>= (Variables|Default|GetAmount%20Players%20overlapped) 2)
    (bind _returnvalue (UserInterface|CreateWidget "/Game/Multiplayer/UI/Fade.Fade_C"))
    (UserInterface|Viewport|AddtoViewport _returnvalue 0)
    (Default|PlayFadein _returnvalue)
    (Utilities|FlowControl|Delay 0.8)
    (Game|OpenLevel(byObjectReference) (Variables|Default|GetNext%20Level))))

(event OnComponentEndOverlap(Trigger)
  (params (OverlappedComponent :type Primitive%20Component%20Object%20Reference) (OtherActor :type Actor%20Object%20Reference) (OtherComp :type Primitive%20Component%20Object%20Reference) (OtherBodyIndex :type Integer))
  (Utilities|Casting|CastToBP_Firefighter OtherActor
    (:then
      (Variables|Default|SetAmount%20Players%20overlapped (- (Variables|Default|GetAmount%20Players%20overlapped) 1)))
    (:CastFailed
      (Utilities|Casting|CastToBP_Astronaut OtherActor)
      (Variables|Default|SetAmount%20Players%20overlapped (- (Variables|Default|GetAmount%20Players%20overlapped) 1)))))

(event EventBeginPlay
  (Utilities|FlowControl|Delay 0.1)
  (for _array_element (Collision|GetOverlappingActors (Variables|Default|GetTrigger) "/Game/Multiplayer/Astronaut/BP_Astronaut.BP_Astronaut_C" :!class /Script/Engine.PrimitiveComponent)
    (Variables|Default|SetAmount%20Players%20overlapped (+ (Variables|Default|GetAmount%20Players%20overlapped) 1))))

(event EventTick
  (params (DeltaSeconds :type Float%20%28single-precision%29)))

(fn ConstructionScript
  (Components|Box|SetBoxExtent (Variables|Default|GetTrigger) (Variables|Default|GetBox%20Extent) true))