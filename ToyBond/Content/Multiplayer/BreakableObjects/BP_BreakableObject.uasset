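; BP_BreakableObject is a breakable prop that swaps its static mesh for a Geometry Collection when BreakObject is called.
; A one-time gate destroys the mesh, then after a short delay adds the collection component and assigns its rest collection.
; A parallel Sequence branch applies a radial impulse if that component exists, so the delay makes the first call skip it.
; Timed actor cleanup and construction-time mesh and scale setup are unconnected.
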(event EventBeginPlay)

(event EventBreakObject
  (Utilities|FlowControl|Sequence
    (:then_0
      (Utilities|FlowControl|DoOnce false
        (:Completed
          (Components|DestroyComponent (Variables|Default|GetStaticMesh))
          (Utilities|FlowControl|Delay 0.05)
          (bind _returnvalue (AddComponent|AddGeometryCollectionComponent false))
          (bind _output_get (Variables|Default|SetNewVar _returnvalue))
          (Class|GeometryCollectionComponent|SetRestCollection _returnvalue (Variables|Default|GetGeometry%20Collection) true))))
    (:then_1
      (bind _newvar (Variables|Default|GetNewVar)
        (:then
          (Class|PhysicsObjectBlueprintLibrary|ApplyRadialImpulse _newvar (Transformation|GetWorldLocation _newvar) 5e+01 5e+05 "RIF_Constant" false 0.0 false 0.0 1.0))
        (:else)))))

(fn ConstructionScript)